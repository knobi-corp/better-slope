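; Procedural map generator actor that keeps appending static mesh segments along the X axis during play.
; A looping timer started on BeginPlay advances a stored transform by the last Offset, then adds one of five randomly chosen mesh components there.
; Each choice sets the Offset for the following segment and prints it for debugging.
; Nothing stops the timer or removes old segments, so components accumulate on the actor.
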(event `self.ReceiveBeginPlay`
  (`KismetSystemLibrary.K2_SetTimerDelegate` (delegate `generate new`) 0.2 true))

(event `generate new`
  (bind _output_get (set `self.old pos` (`KismetMathLibrary.MakeTransform` (`KismetMathLibrary.MakeVector` (+ (.x (.location (`self.old pos`))) (`KismetMathLibrary.Conv_IntToDouble` (`self.offset `))) (.y (.location (`self.old pos`))) (.z (.location (`self.old pos`)))) (.rotation (`self.old pos`)) (.scale (`self.old pos`)))))
  (switch `int` (`KismetMathLibrary.RandomInteger` 5)
    (:`0`
      (`AddComponent|NODE_AddStaticMeshComponent-2` :`RelativeTransform` _output_get)
      (bind _output_get_2 (set `self.offset ` 1500)))
    (:`1`
      (`AddComponent|NODE_AddStaticMeshComponent-3` :`RelativeTransform` _output_get)
      (bind _output_get_3 (set `self.offset ` 2500)))
    (:`2`
      (`AddComponent|NODE_AddStaticMeshComponent-5` :`RelativeTransform` _output_get)
      (bind _output_get_4 (set `self.offset ` 4501)))
    (:`3`
      (`AddComponent|NODE_AddStaticMeshComponent-7` :`RelativeTransform` _output_get)
      (bind _output_get_5 (set `self.offset ` 4501)))
    (:`4`
      (`AddComponent|NODE_AddStaticMeshComponent-8` :`RelativeTransform` _output_get)
      (bind _output_get_6 (set `self.offset ` 4496))))
  (`KismetSystemLibrary.PrintString` (`KismetStringLibrary.Conv_IntToString` _output_get_6)))

(fn `UserConstructionScript`)